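; Look-dev lighting stage actor that builds its environment, sky atmosphere, sun, skylight and post-process in the construction script.
; An optional Config profile overrides the lighting settings first, then update functions apply them, destroying components the chosen mode does not need.
; EV100 drives exposure compensation, HDRI skybox brightness and optional HDRI skylight intensity.
; One Z rotation turns the sun, skybox and HDRI skylight together; a flag toggles Lumen.
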(fn `ApplyProfile`
  (locals (LastLightRotZ :type "Float (double-precision)"))
  (bind _config (`self.Config`))
  (`/Engine/EditorBlueprintResources/StandardMacros.IsValid` (`self.Config`)
    (:`Is Valid`
      (`|ExecutionSequence`
        (:`then_0`
          (set `self.LightRotZInitial` (`/AssetsManager/LookDev/LookDevBP/BP_LookDevConfig.LightRotZInitial` _config)))
        (:`then_1`
          (set `self.UseSkyAtmosphere` (`/AssetsManager/LookDev/LookDevBP/BP_LookDevConfig.UseSkyAtmosphere` _config))
          (set `self.MieScatteringScale` (`/AssetsManager/LookDev/LookDevBP/BP_LookDevConfig.MieScatteringScale` _config))
          (set `self.MieAbsorptionScale` (`/AssetsManager/LookDev/LookDevBP/BP_LookDevConfig.MieAbsorptionScale` _config)))
        (:`then_2`
          (set `self.SkyLightFromHDRI` (`/AssetsManager/LookDev/LookDevBP/BP_LookDevConfig.SkyLightFromHDRI` _config))
          (set `self.HDRI` (`/AssetsManager/LookDev/LookDevBP/BP_LookDevConfig.HDRI` _config))
          (set `self.SkyLight_Intensity` (`/AssetsManager/LookDev/LookDevBP/BP_LookDevConfig.SkyLight_Intensity` _config))
          (set `self.MatchHDRI_SkyLightIntensityToEV100` (`/AssetsManager/LookDev/LookDevBP/BP_LookDevConfig.MatchHDRI_SkyLightIntensityToEV100` _config)))
        (:`then_3`
          (set `self.DirectionalLight_Intensity` (`/AssetsManager/LookDev/LookDevBP/BP_LookDevConfig.DirectionalLight_Intensity` _config))
          (set `self.DirectionalLight_Rotation` (`/AssetsManager/LookDev/LookDevBP/BP_LookDevConfig.DirectionalLight_Rotation` _config))
          (set `self.DirectionalLight_SourceAngle` (`/AssetsManager/LookDev/LookDevBP/BP_LookDevConfig.DirectionalLight_SourceAngle` _config))
          (set `self.DirectionalLight_Temperature` (`/AssetsManager/LookDev/LookDevBP/BP_LookDevConfig.DirectionalLight_Temperature` _config)))
        (:`then_4`
          (set `self.EV100` (`/AssetsManager/LookDev/LookDevBP/BP_LookDevConfig.EV100` _config))
          (set `self.WhiteBalance` (`/AssetsManager/LookDev/LookDevBP/BP_LookDevConfig.WhiteBalance` _config)))))))

(fn `UpdateAtmosphere`
  (bind _skyatmosphere (`self.SkyAtmosphere`))
  (if (`self.UseSkyAtmosphere`)
    (`|ExecutionSequence`
      (:`then_0`
        (`SkyAtmosphereComponent.SetMieScatteringScale` _skyatmosphere (`self.MieScatteringScale`))
        (`SkyAtmosphereComponent.SetMieAbsorptionScale` _skyatmosphere (`self.MieAbsorptionScale`))))
    (else
      (`ActorComponent.K2_DestroyComponent` (`self.SkyAtmosphere`)))))

(fn `UpdateDirectionalLight`
  (bind _directionallight (`self.DirectionalLight`))
  (`SceneComponent.K2_SetWorldRotation` _directionallight (`self.DirectionalLight_Rotation`) false false)
  (`LightComponent.SetIntensity` _directionallight (`self.DirectionalLight_Intensity`))
  (`DirectionalLightComponent.SetLightSourceAngle` _directionallight (`self.DirectionalLight_SourceAngle`))
  (`SceneComponent.K2_AddWorldRotation` _directionallight (`KismetMathLibrary.MakeRotator` 0.0 0.0 (+ (`self.LightRotZInitial`) (`self.LightRotationZ`))) false false)
  (`LightComponent.SetTemperature` _directionallight (`self.DirectionalLight_Temperature`)))

(fn `UpdateEnviroment`
  (locals (MID_GreyBackground :type "MaterialInstanceDynamic Object Reference") (IsGroundShownBefore :type Boolean))
  (bind _ground (`self.Ground`))
  (bind _background (`self.Background`))
  (`|ExecutionSequence`
    (:`then_0`
      (if (`|EnumEquality` _background "NewEnumerator0")
        (`/Engine/EditorBlueprintResources/StandardMacros.IsValid` (`self.HDRI`)
          (:`Is Valid`
            (`self.UpdateSkyBox`)
            (`ActorComponent.K2_DestroyComponent` (`self.ExponentialHeightFog`)))
          (:`Is Not Valid`
            (`ActorComponent.K2_DestroyComponent` (`self.SkyBox`) :!label _label)))
        (else
          (goto _label))))
    (:`then_1`
      (if (`|EnumEquality` _background "NewEnumerator1")
        (bind _returnvalue (`PrimitiveComponent.CreateDynamicMaterialInstance` (`self.GreyBackground`) 0 "/AssetsManager/LookDev/Materials/MI_Gray_NoSpec.MI_Gray_NoSpec" "None"))
        (set `local.MID_GreyBackground` _returnvalue)
        (`ActorComponent.K2_DestroyComponent` (`self.Ground`))
        (`ActorComponent.K2_DestroyComponent` (`self.ExponentialHeightFog`))
        (else
          (`ActorComponent.K2_DestroyComponent` (`self.GreyBackground`)))))
    (:`then_2`
      (if (not (`self.ShowGround`))
        (`/Engine/EditorBlueprintResources/StandardMacros.IsValid` _ground
          (:`Is Valid`
            (`ActorComponent.K2_DestroyComponent` _ground)))))))

(fn `UpdatePostProcess`
  (bind _settings (`PostProcessComponent.Settings` (`self.PostProcess`)))
  (setmembers `PostProcessSettings` :`StructRef` _settings :`WhiteTemp` (`self.WhiteBalance`) :`AutoExposureBias` (+ (* (`self.EV100`) -1.0) (`self.ExposureCompensation`)))
  (if (`self.UseLumen`)
    (setmembers `PostProcessSettings` :`StructRef` _settings :`DynamicGlobalIlluminationMethod` "Lumen" :`ReflectionMethod` "Lumen")
    (else
      (setmembers `PostProcessSettings` :`StructRef` _settings :`DynamicGlobalIlluminationMethod` "None" :`ReflectionMethod` "ScreenSpace"))))

(fn `UpdateSkyBox`
  (locals (MID_SkyBox :type "MaterialInstanceDynamic Object Reference"))
  ;[1 1 1] Create HDRI dynamic material instance
  (bind _returnvalue (`PrimitiveComponent.CreateDynamicMaterialInstance` (`self.SkyBox`) 0 "/AssetsManager/LookDev/Materials/MI_LightStage_Skybox_HDRI.MI_LightStage_Skybox_HDRI" "None"))
  (set `local.MID_SkyBox` _returnvalue)
  ;[1 1 1] HDRI Paraments
  ;;[1 1 1] Assign HDRI cubemap material
  (`MaterialInstanceDynamic.SetTextureParameterValue` (`local.MID_SkyBox`) "HDRI_Cubemap" (`self.HDRI`))
  ;;[1 1 1] Set HDRI Brightness
  (`MaterialInstanceDynamic.SetScalarParameterValue` (`local.MID_SkyBox`) "HDRI_Brightness" (`KismetMathLibrary.MultiplyMultiply_FloatFloat` 2.0 (`self.EV100`)))
  ;;[1 1 1] Apply cubemap rotation (match to BP scene component)
  (`MaterialInstanceDynamic.SetScalarParameterValue` (`local.MID_SkyBox`) "CubemapRotation" (* (`KismetMathLibrary.MapRangeUnclamped` (+ (`self.LightRotZInitial`) (`self.LightRotationZ`)) -360.0 360.0 -1.0 1.0) -1.0)))

(fn `UpdateSkyLight`
  (bind _skylight_hdri (`self.SkyLight_HDRI`))
  (bind _skylight_captured (`self.SkyLight_Captured`))
  (bind _skylight_intensity (`self.SkyLight_Intensity`))
  (if (`self.SkyLightFromHDRI`)
    (`ActorComponent.K2_DestroyComponent` (`self.SkyLight_Captured`))
    (`SkyLightComponent.SetIntensity` _skylight_hdri (select `bool` (`self.MatchHDRI_SkyLightIntensityToEV100`) :`false` _skylight_intensity :`true` (* _skylight_intensity (`KismetMathLibrary.MultiplyMultiply_FloatFloat` 2.0 (`self.EV100`)))))
    (`SkyLightComponent.SetCubemap` _skylight_hdri (`self.HDRI`))
    (`SkyLightComponent.SetSourceCubemapAngle` _skylight_hdri (* (+ (`self.LightRotZInitial`) (`self.LightRotationZ`)) -1.0))
    (`SkyLightComponent.SetLightColor` _skylight_hdri (`self.SkylLight_Color`))
    (else
      (`ActorComponent.K2_DestroyComponent` (`self.SkyLight_HDRI`))
      (`SkyLightComponent.SetIntensity` _skylight_captured (`self.SkyLight_Intensity`))
      (`SkyLightComponent.SetLightColor` _skylight_captured (`self.SkylLight_Color`)))))

(fn `UserConstructionScript`
  (`self.ApplyProfile`)
  (`self.UpdateEnviroment`)
  (`self.UpdateAtmosphere`)
  (`self.UpdateDirectionalLight`)
  (`self.UpdateSkyLight`)
  (`self.UpdatePostProcess`))