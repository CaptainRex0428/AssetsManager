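; Look-dev environment actor for checking assets under low, mid or high contrast lighting, built entirely in the construction script.
; The selected scenario's config drives HDRI, skylight and directional light, with one Z rotation turning lights and skybox together.
; Background mode keeps an HDRI skybox or lit backdrop, destroying unused components and optionally the ground.
; Post process toggles auto exposure and Lumen, and can add a PBR-range checker material.
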(fn `ApplyConfig`
  (locals (LastLightRotZ :type "Float (double-precision)"))
  (bind _config (`self.Config`))
  (bind _output_get (set `self.Config` (select `/AssetsManager/LookDev/Assets/LightingScenarial` (`self.LightScenario`) :`NewEnumerator0` "/AssetsManager/LookDev/LookDevBP/Config/LowContrast.LowContrast" :`NewEnumerator1` "/AssetsManager/LookDev/LookDevBP/Config/MidContrast.MidContrast" :`NewEnumerator2` "/AssetsManager/LookDev/LookDevBP/Config/HighContrast.HighContrast" :!type "/AssetsManager/LookDev/LookDevBP/BP_LookDevConfig Object Reference")))
  (`/Engine/EditorBlueprintResources/StandardMacros.IsValid` _output_get
    (:`Is Valid`
      (`|ExecutionSequence`
        (:`then_0`
          (set `self.HDRI` (`/AssetsManager/LookDev/LookDevBP/BP_LookDevConfig.HDRI` _config))
          (set `self.Sky Light Intensity` (`/AssetsManager/LookDev/LookDevBP/BP_LookDevConfig.Sky Light Intensity` _config))
          (set `self.Sky Light Cast Shadows` (`/AssetsManager/LookDev/LookDevBP/BP_LookDevConfig.Sky Light Cast Shadows` _config)))
        (:`then_1`
          (set `self.Directional Light Intensity` (`/AssetsManager/LookDev/LookDevBP/BP_LookDevConfig.Directional Light Intensity` _config))
          (set `self.Directional Light Rotation` (`/AssetsManager/LookDev/LookDevBP/BP_LookDevConfig.Directional Light Rotation` _config))
          (set `self.Directional Light Source Angle` (`/AssetsManager/LookDev/LookDevBP/BP_LookDevConfig.Directional Light Source Angle` _config)))))))

(fn `PBRCheck`
  (locals (PBRCheckMat :type "MaterialInstanceDynamic Object Reference"))
  (if (`self.PBR Checker`)
    (`|ExecutionSequence`
      (:`then_0`
        (bind _returnvalue (`KismetMaterialLibrary.CreateDynamicMaterialInstance` "/AssetsManager/LookDev/Assets/PBR_Checker_M.PBR_Checker_M"))
        (set `local.PBRCheckMat` _returnvalue)
        (`MaterialInstanceDynamic.SetScalarParameterValue` (`local.PBRCheckMat`) "Max_NoneMetallic" 0.9)
        (`MaterialInstanceDynamic.SetScalarParameterValue` (`local.PBRCheckMat`) "Min_NoneMetallic" 0.02)
        (`MaterialInstanceDynamic.SetScalarParameterValue` (`local.PBRCheckMat`) "Min_Metallic" 0.3))
      (:`then_1`
        (setmembers `PostProcessSettings` :`StructRef` (`PostProcessComponent.Settings` (`self.PostProcess`)) :`WeightedBlendables` (make `WeightedBlendables` (`|MakeArray` (make `WeightedBlendable` 1.0 (`local.PBRCheckMat`)))))))))

(fn `UpdateDirectionalLight`
  (`SceneComponent.K2_SetWorldRotation` (`self.DirectionalLight`) (`self.Directional Light Rotation`) false false)
  (`LightComponent.SetIntensity` (`self.DirectionalLight`) (`self.Directional Light Intensity`))
  (`DirectionalLightComponent.SetLightSourceAngle` (`self.DirectionalLight`) (`self.Directional Light Source Angle`))
  (`SceneComponent.K2_AddWorldRotation` (`self.DirectionalLight`) (`KismetMathLibrary.MakeRotator` 0.0 0.0 (`self.Light RotationZ`)) false false))

(fn `UpdatePostProcess`
  (bind _settings (`PostProcessComponent.Settings` (`self.PostProcess`)))
  (bind _settings_2 (`PostProcessComponent.Settings` (`self.PostProcess`)))
  (if (`self.Auto Exposure`)
    (setmembers `PostProcessSettings` :`StructRef` _settings :`AutoExposureMethod` "AEM_Histogram" :`AutoExposureBias` (`self.Exposure Compensation`) :`AutoExposureApplyPhysicalCameraExposure` true)
    (else
      (setmembers `PostProcessSettings` :`StructRef` _settings :`AutoExposureMethod` "AEM_Manual" :`AutoExposureBias` (`self.Exposure Compensation`) :`AutoExposureApplyPhysicalCameraExposure` false)))
  (if (`self.Use Lumen`)
    (setmembers `PostProcessSettings` :`StructRef` _settings_2 :`DynamicGlobalIlluminationMethod` "Lumen" :`ReflectionMethod` "Lumen")
    (else
      (setmembers `PostProcessSettings` :`StructRef` _settings_2 :`DynamicGlobalIlluminationMethod` "None" :`ReflectionMethod` "ScreenSpace")))
  (`self.PBRCheck`))

(fn `UpdateSkyBox`
  (locals (MID_SkyBox :type "MaterialInstanceDynamic Object Reference"))
  ;[1 1 1] Create HDRI dynamic material instance
  (bind _returnvalue (`PrimitiveComponent.CreateDynamicMaterialInstance` (`self.SkyBox`) 0 "/AssetsManager/LookDev/Assets/Materials/M_LightStage_Skybox_HDRI.M_LightStage_Skybox_HDRI" "None"))
  (set `local.MID_SkyBox` _returnvalue)
  ;[1 1 1] HDRI Paraments
  ;;[1 1 1] Assign HDRI cubemap material
  (`MaterialInstanceDynamic.SetTextureParameterValue` (`local.MID_SkyBox`) "HDRI_Cubemap" (`self.HDRI`))
  ;;[1 1 1] Set HDRI Brightness
  (`MaterialInstanceDynamic.SetScalarParameterValue` (`local.MID_SkyBox`) "HDRI_Brightness" (`KismetMathLibrary.MultiplyMultiply_FloatFloat` 2.0))
  ;;[1 1 1] Apply cubemap rotation (match to BP scene component)
  (`MaterialInstanceDynamic.SetScalarParameterValue` (`local.MID_SkyBox`) "CubemapRotation" (* (`KismetMathLibrary.MapRangeUnclamped` (+ (`self.Light RotZ Initial`) (`self.Light RotationZ`)) -360.0 360.0 -1.0 1.0) -1.0)))

(fn `UpdateSkyLight`
  (`SkyLightComponent.SetIntensity` (`self.SkyLight_HDRI`) (`self.Sky Light Intensity`))
  (`SkyLightComponent.SetCubemap` (`self.SkyLight_HDRI`) (`self.HDRI`))
  (`SkyLightComponent.SetSourceCubemapAngle` (`self.SkyLight_HDRI`) (* (`self.Light RotationZ`) -1.0))
  (`LightComponentBase.SetCastShadows` (`self.SkyLight_HDRI`) (`self.Sky Light Cast Shadows`)))

(fn `UpdateWorld`
  (locals (MID_LitBackground :type "MaterialInstanceDynamic Object Reference") (IsGroundShownBefore :type Boolean))
  (bind _ground (`self.Ground`))
  (bind _background (`self.Background`))
  (`|ExecutionSequence`
    (:`then_0`
      (if (`|EnumEquality` _background "NewEnumerator0")
        (`/Engine/EditorBlueprintResources/StandardMacros.IsValid` (`self.HDRI`)
          (:`Is Valid`
            (`self.UpdateSkyBox`))
          (:`Is Not Valid`
            (`ActorComponent.K2_DestroyComponent` (`self.SkyBox`) :!label _label)))
        (else
          (goto _label))))
    (:`then_1`
      (if (`|EnumEquality` _background "NewEnumerator1")
        (bind _returnvalue (`PrimitiveComponent.CreateDynamicMaterialInstance` (`self.LitBackground`) 0 "/AssetsManager/LookDev/Assets/Gray_NoSpec.Gray_NoSpec" "None"))
        (set `local.MID_LitBackground` _returnvalue)
        (`ActorComponent.K2_DestroyComponent` (`self.Ground`))
        (elif (`|EnumEquality` (`self.Background`) "NewEnumerator3")
          (bind _returnvalue_2 (`PrimitiveComponent.CreateDynamicMaterialInstance` (`self.LitBackground`) 0 "/AssetsManager/LookDev/Assets/Gray_NoSpec.Gray_NoSpec" "None"))
          (bind _output_get (set `local.MID_LitBackground` _returnvalue_2))
          (`MaterialInstanceDynamic.SetScalarParameterValue` _output_get "BaseColor" 0.02)
          (`ActorComponent.K2_DestroyComponent` (`self.Ground`))
          (else
            (`ActorComponent.K2_DestroyComponent` (`self.LitBackground`))))))
    (:`then_2`
      (if (not (`self.Show Ground`))
        (`/Engine/EditorBlueprintResources/StandardMacros.IsValid` _ground
          (:`Is Valid`
            (`ActorComponent.K2_DestroyComponent` _ground)))))))

(fn `UserConstructionScript`
  (`self.ApplyConfig`)
  (`self.UpdateWorld`)
  (`self.UpdateDirectionalLight`)
  (`self.UpdateSkyLight`)
  (`self.UpdatePostProcess`))